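; Game mode for Animal Guys that tracks player count, controls the Falling Level's waiting wall and handles match finish.
; New players update current and remaining counts in the game state.
; BeginPlay caches the wall on the Falling Level; CallBreakWall starts a Tick timer that destroys it after WaitingTime.
; ProcessFinish resets character stats and moves winners to a tagged target point, while losers' target lookup goes unused.
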(event EventBeginPlay
  (bind _returnvalue (Game|GetCurrentLevelName true))
  (switch string _returnvalue
    (:AnimalGuys_MainGameFallingLevel
      (CallFunction|PrepareFallingLevel))))

(event EventHandleStartingNewPlayer
  (params (NewPlayer :type Player%20Controller%20Object%20Reference))
  (|CallParentFunction NewPlayer)
  (bind _returnvalue (Class|GameModeBase|GetNumPlayers))
  (bind _output_get (Variables|Default|SetCurPlayerCount _returnvalue))
  (bind _asbp_animal_guys_game_state (Utilities|Casting|CastToBP_AnimalGuys_GameState (Game|GetGameState)))
  (Default|SetCurPlayerCount _asbp_animal_guys_game_state _output_get)
  (Default|SetLeftPlayerCount _asbp_animal_guys_game_state _output_get))

(event EventPostLogin
  (params (NewPlayer :type Player%20Controller%20Object%20Reference))
  ;[1 1 1] Event Handle Starting New Player와 유사하게 작동함[사용하지 않음]
)

(event EventTick
  (params (DeltaSeconds :type Float%20%28single-precision%29))
  (bind _waitingwall (Variables|Default|GetWaitingWall))
  (if (Variables|Default|GetbBreakWallCall)
    (bind _output_get (Variables|Default|SetElapsedTime (+ DeltaSeconds (Variables|Default|GetElapsedTime))))
    (if (> _output_get (Variables|Default|GetWaitingTime))
      (Variables|Default|SetbBreakWallCall false)
      (Utilities|IsValid _waitingwall
        (:Is%20Valid
          (Actor|DestroyActor _waitingwall))))))

(fn ConstructionScript)

(fn CallBreakWall
  (Variables|Default|SetbBreakWallCall true)
  (Variables|Default|SetElapsedTime 0.0))

(fn ProcessFinish
  (params (WinCharArray :type Array%20of%20BP%20Animal%20Guys%20Character%20Object%20References) (LoseCharArray :type Array%20of%20BP%20Animal%20Guys%20Character%20Object%20References))
  (Utilities|FlowControl|Sequence
    (:then_0
      (for _array_element WinCharArray
        (Default|CharacterStat _array_element 30 0 0 0.0 0.0 0.0 1e+02 3.0 5.0)
        (bind _outactors (Actor|GetAllActorsOfClasswithTag "/Script/Engine.Actor" "WinnerTargetPoint"))
        (Transformation|SetActorLocation _array_element (Transformation|GetActorLocation (Utilities|Array|Get(acopy) _outactors)) false false)))
    (:then_1
      (for _array_element_2 LoseCharArray
        (Default|CharacterStat _array_element_2 30 0 0 0.0 0.0 0.0 1e+02 3.0 5.0)
        (Actor|GetAllActorsOfClasswithTag "/Script/Engine.Actor" "LoserTargetPoint")))))

(fn PrepareFallingLevel
  (bind _returnvalue (Actor|GetActorOfClass "/Game/AnimalGuys/3_KangHoJae/Levels/GamePlay/Blueprint/BP_WaitingWall.BP_WaitingWall_C"))
  (Utilities|IsValid _returnvalue
    (:Is%20Valid
      (Variables|Default|SetWaitingWall _returnvalue)
      (Development|PrintString "BP_WaitingWall Exists!"))
    (:Is%20Not%20Valid
      (Development|PrintString "BP_WaitingWall Not Exists!"))))